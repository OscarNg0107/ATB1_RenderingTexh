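; BP_Botan is a character Blueprint that detects whether Botan is shadowed from the direct light and publishes the result to the MPC_LightSource material parameter collection.
; Each Tick it traces along the DirectLight vector, easing the Visibility hit result into that parameter's alpha and writing a second channel's raw hit to Blocked.
; The construction script runs similar logic, using one Visibility trace for both values.
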(event `self.ReceiveTick`
  (params (DeltaSeconds :type "Float (single-precision)"))
  (bind _returnvalue (+ (`self.K2_GetActorLocation`) (0.0 0.0 10.0)))
  (bind _returnvalue_2 (`KismetMaterialLibrary.GetVectorParameterValue` "/Game/CustomMaterial/MPC_LightSource.MPC_LightSource" "DirectLight"))
  (bind _returnvalue_3 (+ _returnvalue (* _returnvalue_2 (`self.Light Trace Length`))))
  (bind (_outhit _returnvalue_4) (`KismetSystemLibrary.LineTraceSingle` _returnvalue _returnvalue_3 "TraceTypeQuery1"))
  (bind (_r _g _b _a) (break `LinearColor` _returnvalue_2))
  (`KismetMaterialLibrary.SetVectorParameterValue` "/Game/CustomMaterial/MPC_LightSource.MPC_LightSource" "DirectLight" (make `LinearColor` _r _g _b (`KismetMathLibrary.FInterpTo` _a (`KismetMathLibrary.Conv_BoolToDouble` _returnvalue_4) (`GameplayStatics.GetWorldDeltaSeconds`) 30.0)))
  (bind (_outhit_2 _returnvalue_5) (`KismetSystemLibrary.LineTraceSingle` _returnvalue _returnvalue_3 "TraceTypeQuery3"))
  (`KismetMaterialLibrary.SetScalarParameterValue` "/Game/CustomMaterial/MPC_LightSource.MPC_LightSource" "Blocked" (`KismetMathLibrary.Conv_BoolToDouble` _returnvalue_5)))

(fn `UserConstructionScript`
  (bind _returnvalue (+ (`self.K2_GetActorLocation`) (0.0 0.0 10.0)))
  (bind _returnvalue_2 (`KismetMaterialLibrary.GetVectorParameterValue` "/Game/CustomMaterial/MPC_LightSource.MPC_LightSource" "DirectLight"))
  (bind (_outhit _returnvalue_3) (`KismetSystemLibrary.LineTraceSingle` _returnvalue (+ _returnvalue (* _returnvalue_2 (`self.Light Trace Length`))) "TraceTypeQuery1"))
  (bind _returnvalue_4 (`KismetMathLibrary.Conv_BoolToDouble` _returnvalue_3))
  (`KismetMaterialLibrary.SetScalarParameterValue` "/Game/CustomMaterial/MPC_LightSource.MPC_LightSource" "Blocked" _returnvalue_4)
  (bind (_r _g _b _a) (break `LinearColor` _returnvalue_2))
  (`KismetMaterialLibrary.SetVectorParameterValue` "/Game/CustomMaterial/MPC_LightSource.MPC_LightSource" "DirectLight" (make `LinearColor` _r _g _b (`KismetMathLibrary.FInterpTo` _a _returnvalue_4 (`GameplayStatics.GetWorldDeltaSeconds`) 30.0))))