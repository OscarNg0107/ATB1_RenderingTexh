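; BP_DirectLight publishes the direction of a directional light to materials through the MPC_LightSource material parameter collection.
; It negates the DirectionalLight forward vector to point toward the light and writes it to the DirectLight vector parameter.
; The write runs in the construction script, so it refreshes on placement or edit, and again every Tick to follow rotation at runtime.
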(event `self.ReceiveTick`
  (params (DeltaSeconds :type "Float (single-precision)"))
  (`KismetMaterialLibrary.SetVectorParameterValue` "/Game/CustomMaterial/MPC_LightSource.MPC_LightSource" "DirectLight" (`KismetMathLibrary.Conv_VectorToLinearColor` (* (`SceneComponent.GetForwardVector` (`self.DirectionalLight`)) -1.0))))

(fn `UserConstructionScript`
  (`KismetMaterialLibrary.SetVectorParameterValue` "/Game/CustomMaterial/MPC_LightSource.MPC_LightSource" "DirectLight" (`KismetMathLibrary.Conv_VectorToLinearColor` (* (`SceneComponent.GetForwardVector` (`self.DirectionalLight`)) (-1.0 -1.0 -1.0)))))